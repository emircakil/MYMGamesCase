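; BP_CarpenterGameState is the game state for a carpenter game, holding the current customer-style order of an item type and color.
; On BeginPlay, the server starts a self-recalling loop that rolls a random order, prints it for debugging, and repeats after a random delay.
; The CurrentOrder RepNotify finds the BP_OrderBoard actor and passes the order to its WBP_OrderBoard widget to update the display.
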(event Custom|GenerateNewOrder
  (bind _output_get (Variables|Default|SetCurrentOrder (Utilities|Struct|MakeF_OrderData (Utilities|Enum|ByteToEnumE_ItemType (Math|Conversions|ToByte(Integer) (Math|Random|RandomIntegerinRange 0 3))) (Utilities|Enum|ByteToEnumE_ItemColor (Math|Conversions|ToByte(Integer) (Math|Random|RandomIntegerinRange 0 3))))))
  (Development|PrintString (Utilities|String|EnumtoString (.itemtype _output_get)))
  (Development|PrintString (Utilities|String|EnumtoString (.itemcolor _output_get)))
  ;[0.15 0.15 0.15 0.5] Re generate ranom item in random time - recursive call
  (Utilities|FlowControl|Delay (Math|Random|RandomFloatinRange 1e+01 25.0))
  (CallFunction|GenerateNewOrder))

(event EventBeginPlay
  (Networking|SwitchHasAuthority
    (:Authority
      (CallFunction|GenerateNewOrder))))

(fn ConstructionScript)

(fn OnRepCurrentOrder
  (bind _returnvalue (Actor|GetActorOfClass "/Game/CarpenterGame/Core/Interactables/BP_OrderBoard.BP_OrderBoard_C"))
  (bind _aswbp_order_board (Utilities|Casting|CastToWBP_OrderBoard (UserInterface|GetWidget (Variables|/Game/CarpenterGame/Core/Interactables/BP_OrderBoard.BP_OrderBoard_C|GetWidget _returnvalue))))
  (Default|UpdateOrderUI _aswbp_order_board (Variables|Default|GetCurrentOrder)))