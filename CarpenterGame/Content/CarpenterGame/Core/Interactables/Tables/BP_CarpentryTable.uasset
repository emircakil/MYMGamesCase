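; BP_CarpentryTable is an interactable table that turns placed raw wood into a crafted item.
; Placing a BP_RawWood on it stores the reference and sets HasWood, which lets Interact open WBP_CraftMenu on the player's client.
; StartCrafting clears the flag, destroys the wood and spawns the chosen class at the PlacementPoint transform.
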(event Custom|StartCrafting
  (params (ClassToSpawn :type Actor%20Class%20Reference))
  (bind _placementpoint (Variables|Default|GetPlacementPoint))
  (if (Variables|Default|GetbHasWood)
    (Variables|Default|SetbHasWood false)
    (Actor|DestroyActor (Variables|Default|GetAs%20BP%20Raw%20Wood))
    (Game|SpawnActorfromClass ClassToSpawn (Math|Transform|MakeTransform (Transformation|GetWorldLocation _placementpoint) (Transformation|GetWorldRotation _placementpoint) "1.000000,1.000000,1.000000") "AdjustIfPossibleButAlwaysSpawn" "MultiplyWithRoot" 0 0)))

(event EventInteract
  (params (Player :type BP%20Carpenter%20Character%20Object%20Reference))
  (|CallParentFunction Player)
  (if (Variables|Default|GetbHasWood)
    (Default|ClientOpenCraftMenu Player self "/Game/CarpenterGame/Core/UI/WBP_CraftMenu.WBP_CraftMenu_C")))

(fn ConstructionScript
  (|CallParentFunction))

(fn OnItemPlaced
  (params (PlacedItem :type Actor%20Object%20Reference))
  (|CallParentFunction PlacedItem)
  (Utilities|IsValid PlacedItem
    (:Is%20Valid
      (bind _asbp_raw_wood (Utilities|Casting|CastToBP_RawWood PlacedItem)
        (:then
          (Variables|Default|SetAs%20BP%20Raw%20Wood _asbp_raw_wood)
          (Variables|Default|SetbHasWood true))
        (:CastFailed
          (Development|PrintString "No RawWoodItem" true true "(R=1.000000,G=0.039642,B=0.550805,A=1.000000)"))))))