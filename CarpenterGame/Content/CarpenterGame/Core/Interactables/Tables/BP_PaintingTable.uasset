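; Painting table interactable that lets a player recolor a furniture item placed on it.
; OnItemPlaced stores a valid item and flags the table as occupied, so Interact has the player open the paint menu client-side, passing this table along.
; StartPainting casts the stored item to BP_FurnitureItemBase, sets its ItemColor to the new color and clears the occupied flag.
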(event Custom|StartPainting
  (params (NewColor :type E_ItemColor%20Enum :default "NewEnumerator4"))
  (bind _asbp_furniture_item_base (Utilities|Casting|CastToBP_FurnitureItemBase (Variables|Default|GetPlaced%20Item)))
  (Variables|/Game/CarpenterGame/Core/Interactables/Bases/BP_FurnitureItemBase.BP_FurnitureItemBase_C|SetItemColor _asbp_furniture_item_base NewColor)
  (Variables|Default|SetHasITem false))

(event EventInteract
  (params (Player :type BP%20Carpenter%20Character%20Object%20Reference))
  (|CallParentFunction Player)
  (if (Variables|Default|GetHasITem)
    (Default|ClientOpenCraftMenu Player self "/Game/CarpenterGame/Core/UI/WBP_PaintMenu.WBP_PaintMenu_C")))

(fn ConstructionScript
  (|CallParentFunction))

(fn OnItemPlaced
  (params (PlacedItem :type Actor%20Object%20Reference))
  (|CallParentFunction PlacedItem)
  (Utilities|IsValid PlacedItem
    (:Is%20Valid
      (Variables|Default|SetPlaced%20Item PlacedItem)
      (Variables|Default|SetHasITem true))))