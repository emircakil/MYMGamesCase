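; Order table that takes furniture items placed on it and checks them against the current order in the carpenter game state, on the server only.
; It looks first for an entry matching both type and color, then for one matching type only.
; Either match removes that entry, while no match removes the first entry instead.
; In every case the placed item is destroyed and the order is written back to the game state.
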(event EventBeginPlay)

(event Collision|EventActorBeginOverlap
  (params (OtherActor :type Actor%20Object%20Reference)))

(event EventTick
  (params (DeltaSeconds :type Float%20%28single-precision%29)))

(fn ConstructionScript
  (|CallParentFunction))

(fn OnItemPlaced
  (params (PlacedItem :type Actor%20Object%20Reference))
  (|CallParentFunction PlacedItem)
  (Networking|SwitchHasAuthority
    (:Authority
      (Variables|Default|SetisPerfectMatch false)
      (Variables|Default|SetisHalfMatch false)
      (Utilities|IsValid PlacedItem
        (:Is%20Valid
          (bind _asbp_furniture_item_base (Utilities|Casting|CastToBP_FurnitureItemBase PlacedItem))
          (bind _asbp_carpenter_game_state (Utilities|Casting|CastToBP_CarpenterGameState (Game|GetGameState)))
          (Variables|Default|SetAs%20BP%20Carpenter%20Game%20State _asbp_carpenter_game_state)
          (CallFunction|CheckPerfectMatch (Variables|/Game/CarpenterGame/Core/GameModes/BP_CarpenterGameState.BP_CarpenterGameState_C|GetCurrentOrder _asbp_carpenter_game_state) _asbp_furniture_item_base)
          (if (not (Variables|Default|GetisPerfectMatch))
            (CallFunction|CheckHalfMatch (Variables|/Game/CarpenterGame/Core/GameModes/BP_CarpenterGameState.BP_CarpenterGameState_C|GetCurrentOrder _asbp_carpenter_game_state) _asbp_furniture_item_base)
            (if (not (Variables|Default|GetisHalfMatch))
              (Development|PrintString "No item match")
              (Utilities|Array|RemoveIndex (Variables|/Game/CarpenterGame/Core/GameModes/BP_CarpenterGameState.BP_CarpenterGameState_C|GetCurrentOrder _asbp_carpenter_game_state))
              (Actor|DestroyActor _asbp_furniture_item_base)
              (Variables|/Game/CarpenterGame/Core/GameModes/BP_CarpenterGameState.BP_CarpenterGameState_C|SetCurrentOrder (Variables|Default|GetAs%20BP%20Carpenter%20Game%20State) (Variables|/Game/CarpenterGame/Core/GameModes/BP_CarpenterGameState.BP_CarpenterGameState_C|GetCurrentOrder _asbp_carpenter_game_state)))))))))

(fn CheckPerfectMatch
  (params (CurrentItems :type Array%20of%20F%20Order%20Data%20Structures) (FurnitureItem :type BP%20Furniture%20Item%20Base%20Object%20Reference))
  (for (_array_element _array_index) CurrentItems
    (if (and (Utilities|Enum|Equal(Enum) (.itemtype _array_element) (Variables|/Game/CarpenterGame/Core/Interactables/Bases/BP_FurnitureItemBase.BP_FurnitureItemBase_C|GetItemType FurnitureItem)) (Utilities|Enum|Equal(Enum) (.itemcolor _array_element) (Variables|/Game/CarpenterGame/Core/Interactables/Bases/BP_FurnitureItemBase.BP_FurnitureItemBase_C|GetItemColor FurnitureItem)))
      (Development|PrintString "Perfect Item Match")
      (Utilities|Array|RemoveIndex CurrentItems _array_index)
      (Variables|Default|SetisPerfectMatch true)
      (Actor|DestroyActor FurnitureItem)
      (Variables|/Game/CarpenterGame/Core/GameModes/BP_CarpenterGameState.BP_CarpenterGameState_C|SetCurrentOrder (Variables|Default|GetAs%20BP%20Carpenter%20Game%20State) CurrentItems)
      (return))))

(fn CheckHalfMatch
  (params (CurrentItems :type Array%20of%20F%20Order%20Data%20Structures) (FurnitureItem :type BP%20Furniture%20Item%20Base%20Object%20Reference))
  (for (_array_element _array_index) CurrentItems
    (if (Utilities|Enum|Equal(Enum) (.itemtype _array_element) (Variables|/Game/CarpenterGame/Core/Interactables/Bases/BP_FurnitureItemBase.BP_FurnitureItemBase_C|GetItemType FurnitureItem))
      (Development|PrintString "Hald Item Match")
      (Utilities|Array|RemoveIndex CurrentItems _array_index)
      (Variables|Default|SetisHalfMatch true)
      (Actor|DestroyActor FurnitureItem)
      (Variables|/Game/CarpenterGame/Core/GameModes/BP_CarpenterGameState.BP_CarpenterGameState_C|SetCurrentOrder (Variables|Default|GetAs%20BP%20Carpenter%20Game%20State) CurrentItems)
      (return))))