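; BP_PlaceAreaBase is a base interactable where a player puts down the held object at a placement point.
; Interact detaches and teleports the object locally first to hide detach lag, then has the player send the placement transform to the server.
; It finally calls OnItemPlaced with the object, which here only prints it.
; The construction script and HeldObject rep-notify are empty.
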(event EventInteract
  (params (Player :type BP%20Carpenter%20Character%20Object%20Reference))
  (bind _heldobject (Variables|/Game/CarpenterGame/Core/Characters/BP_CarpenterCharacter.BP_CarpenterCharacter_C|GetHeldObject Player))
  (bind _placementpoint (Variables|Default|GetPlacementPoint))
  ;[0.15 0.15 0.15 0.5] First - Detach object on client - solves to detach lag for server
  (Variables|Default|SetPlacedObject _heldobject)
  (Transformation|DetachFromActor _heldobject "KeepWorld" "KeepWorld" "KeepWorld")
  (Transformation|SetActorLocationAndRotation _heldobject (Transformation|GetWorldLocation _placementpoint) (Transformation|GetWorldRotation _placementpoint) false true)
  ;[0.15 0.15 0.15 0.5] Second - Detach object on server
  (Default|ServerPlaceItemtoArea Player (Transformation|GetWorldTransform (Variables|Default|GetPlacementPoint)))
  (CallFunction|OnItemPlaced (Variables|Default|GetPlacedObject)))

(fn ConstructionScript)

(fn OnRepHeldObject)

(fn OnItemPlaced
  (params (PlacedItem :type Actor%20Object%20Reference))
  (Development|PrintString (Utilities|String|ToString(Object) PlacedItem)))